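; Base actor for a world-space UI panel that can face the camera and be grabbed by its border.
; Each Tick, when LookAtTheCamera is set, the Widget component turns toward the player camera on yaw only, staying upright.
; When Draggable, the Draagable function tests whether the interaction pointer's 2D hit lies within the edge margins, then attaches to that WidgetInteractionComponent and moves the actor to the hit location.
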(event EventBeginPlay)

(event Collision|EventActorBeginOverlap
  (params (OtherActor :type Actor%20Object%20Reference)))

(event EventTick
  (params (DeltaSeconds :type Float%20%28single-precision%29))
  (if (Variables|Default|GetLook%20at%20the%20camera)
    (Transformation|SetWorldRotation (Variables|Default|GetWidget) (Math|Rotator|MakeRotator 0.0 0.0 (.yaw (Math|Rotator|FindLookatRotation (Transformation|GetWorldLocation (Variables|Default|GetWidget)) (Camera|GetCameraLocation (Game|GetPlayerCameraManager 0))))) false false)))

(fn ConstructionScript)

(fn Draagable
  (params (WidgetInteractionComponent :type Widget%20Interaction%20Component%20Object%20Reference))
  (bind _returnvalue (Class|WidgetInteractionComponent|Get2DHitLocation WidgetInteractionComponent))
  (bind _panlex (Variables|Default|GetPanleX))
  (bind _panley (Variables|Default|GetPanleY))
  (bind _widget (Variables|Default|GetWidget))
  (bind _returnvalue_2 (Class|WidgetComponent|GetDrawSize _widget))
  (if (Variables|Default|GetbDraggable)
    (if (Math|Boolean|ORBoolean (<= (.x _returnvalue) _panlex) (>= (.x _returnvalue) (- (.x _returnvalue_2) _panlex)) (<= (.y _returnvalue) _panley) (>= (.y _returnvalue) (- (.y _returnvalue_2) _panley)))
      (Transformation|AttachComponentToComponent self WidgetInteractionComponent "None" "KeepRelative" "KeepRelative" "KeepRelative" true)
      (Transformation|SetActorLocation self (.Location (Collision|BreakHitResult (Class|WidgetInteractionComponent|GetLastHitResult WidgetInteractionComponent))) false false))))
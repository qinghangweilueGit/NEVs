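; BP_ItemActor is a VR-grabbable item built from nested child item actors that can split apart and reassemble, apparently for car parts.
; MeetingAndParting computes one of three half-circle layouts, and each child moves along it through the Excursion timeline.
; A camera-facing name widget with a Niagara line labels each item.
; Helpers handle child collision, custom-depth highlighting, see-through material state, reattachment on release and reset to spawn transforms.
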(event EventBeginPlay
  (initialize|Initialize))

(event Collision|EventActorBeginOverlap
  (params (OtherActor :type Actor%20Object%20Reference)))

(event EventTick
  (params (DeltaSeconds :type Float%20%28single-precision%29))
  (bind _widget (Variables|Default|GetWidget))
  (bind _returnvalue (Transformation|GetWorldLocation _widget))
  (Utilities|FlowControl|Sequence
    (:then_0
      (CallFunction|SetWidgetWorldRotator)
      (if (Variables|/Script/Engine.SceneComponent|GetbVisible (Variables|Default|GetNiagara))
        (Class|NiagaraDataInterfaceArrayFunctionLibrary|SetNiagaraArrayVector (Variables|Default|GetNiagara) "User.PointArray" (Utilities|Array|MakeArray _returnvalue _returnvalue _returnvalue _returnvalue (Transformation|GetWorldLocation (Variables|Default|GetStaticMesh))))))
    (:then_1
      (if true
        (Development|PrintString (Utilities|String|Append (Utilities|String|ToString(Vector) (.location (Variables|MeetingAndParting|GetDefaultTransform))) "__" (Utilities|String|ToString(Vector) (.location (Variables|MeetingAndParting|GetSkewTransform))) "__" (Utilities|String|ToString(Vector) (Transformation|GetActorLocation))) true true "(R=0.000000,G=0.660000,B=1.000000,A=1.000000)" 0.0)))))

(event EventIGrab
  (params (MotionControllerComponent :type Motion%20Controller%20Component%20Object%20Reference) (StaticMesh :type Static%20Mesh%20Component%20Object%20Reference) (SkeletalMesh :type Skeletal%20Mesh%20Component%20Object%20Reference) (GrabActor :type Actor%20Object%20Reference) (BoneSlotName :type Name :default "None"))
  (Utilities|IsValid MotionControllerComponent
    (:Is%20Valid
      (Transformation|AttachComponentToComponent self MotionControllerComponent "None" "KeepWorld" "KeepWorld" "KeepWorld" true))))

(event EventIRelease
  (params (MotionControllerComponent :type Motion%20Controller%20Component%20Object%20Reference) (StaticMesh :type Static%20Mesh%20Component%20Object%20Reference) (SkeletalMesh :type Skeletal%20Mesh%20Component%20Object%20Reference))
  (Transformation|DetachFromActor self "KeepWorld" "KeepWorld" "KeepWorld")
  (CallFunction|AttachtoParentActor))

(fn ConstructionScript)

(fn GetThisChildActors
  (for _array_element (Actor|GetComponentsByClass "/Script/Engine.ChildActorComponent")
    (Utilities|Array|Add (LocalVariables|GetLocaldActors) (Variables|/Script/Engine.ChildActorComponent|GetChildActor _array_element)))
  (return (LocalVariables|GetLocaldActors)))

(fn SetThisSubItemActorCollision
  (params (CollisionEnabled :type ECollisionEnabled%20Enum :default "NoCollision"))
  (for _array_element (Actor|GetComponentsByClass "/Script/Engine.ChildActorComponent")
    (bind _asbp_item_actor (Utilities|Casting|CastToBP_ItemActor (Variables|/Script/Engine.ChildActorComponent|GetChildActor _array_element)))
    (for _array_element_2 (Actor|GetComponentsByClass _asbp_item_actor "/Script/Engine.StaticMeshComponent")
      (Collision|SetCollisionEnabled _array_element_2 CollisionEnabled))))

(fn GetRelativeCoordinates
  (params (Locations :type Array%20of%20Vectors))
  (for _array_element Locations
    (Utilities|Array|Add (LocalVariables|GetLoadLocationarray) (- _array_element (Transformation|GetActorLocation self))))
  (return (LocalVariables|GetLoadLocationarray)))

(fn Perspective
  (params (Enable%20perspective :type Boolean))
  (if Enable%20perspective
    (Variables|Perspective|SetCognitiveIndex 1)
    (bind _subactor (CallFunction|GetThisChildActors))
    (for _array_element _subactor
      (bind _asbp_item_actor (Utilities|Casting|CastToBP_ItemActor _array_element))
      (Variables|BP_ItemActor_C|SetCognitiveIndex _asbp_item_actor 1))
    (else
      (Variables|Perspective|SetCognitiveIndex 0)
      (bind _subactor_2 (CallFunction|GetThisChildActors))
      (for _array_element_2 _subactor_2
        (bind _asbp_item_actor_2 (Utilities|Casting|CastToBP_ItemActor _array_element_2))
        (Perspective|SetMeshPerspective _asbp_item_actor_2 false)
        (Variables|BP_ItemActor_C|SetCognitiveIndex _asbp_item_actor_2 0))
      (Perspective|SetMeshPerspective false))))

(fn SetMeshPerspective
  (params (Perspective :type Boolean))
  (bind _staticmesh (Variables|Default|GetStaticMesh))
  (bind _returnvalue (Rendering|Material|GetMaterials _staticmesh))
  (if Perspective
    (Variables|Perspective|SetDefaultMaterial _returnvalue)
    (for (_ _array_index) _returnvalue
      (Rendering|Material|SetMaterial (Variables|Default|GetStaticMesh) _array_index (Variables|Perspective|GetMI_Perspective))
      (Collision|SetCollisionEnabled (Variables|Default|GetStaticMesh) "NoCollision"))
    (else
      (for (_ _array_index_2) (Rendering|Material|GetMaterials (Variables|Default|GetStaticMesh))
        (Rendering|Material|SetMaterial (Variables|Default|GetStaticMesh) _array_index_2 (Utilities|Array|Get(acopy) (Variables|Perspective|GetDefaultMaterial) _array_index_2))
        (Collision|SetCollisionEnabled (Variables|Default|GetStaticMesh) "QueryAndPhysics")))))

(fn SetsAllOfItselfandItsChildrenStaticMesh
  (params (Value :type Boolean))
  (Utilities|FlowControl|Sequence
    (:then_0
      (for _array_element (Actor|GetComponentsByClass "/Script/Engine.StaticMeshComponent")
        (Rendering|SetRenderCustomDepth _array_element Value)))
    (:then_1
      (for _array_element_2 (Actor|GetComponentsByClass "/Script/Engine.ChildActorComponent")
        (Utilities|IsValid _array_element_2
          (:Is%20Valid
            (bind _asbp_item_actor (Utilities|Casting|CastToBP_ItemActor (Variables|/Script/Engine.ChildActorComponent|GetChildActor _array_element_2)))
            (CallFunction|SetsAllOfItselfandItsChildrenStaticMesh _asbp_item_actor Value)
            (for _array_element_3 (Actor|GetComponentsByClass _asbp_item_actor "/Script/Engine.StaticMeshComponent")
              (Rendering|SetRenderCustomDepth _array_element_3 Value))))))))

(fn Initialize
  (bind _self self)
  (bind _self_2 self)
  (bind _returnvalue (Transformation|GetActorTransform _self_2))
  (bind _returnvalue_2 (Actor|GetParentActor _self))
  (Initialize|InitializeUMG)
  (Variables|Default|SetThisSpawnTransform _returnvalue)
  (Variables|MeetingAndParting|SetDefaultTransform _returnvalue)
  (Utilities|IsValid _returnvalue_2
    (:Is%20Valid
      (Variables|Default|SetParentActor _returnvalue_2))))

(fn InitializeUMG
  (bind _returnvalue (UserInterface|CreateWidget "/Game/N_UI/Moudle_1/UMG_ItemNameButton.UMG_ItemNameButton_C" 0 (Variables|ItemData|GetItemActorID)))
  (UserInterface|SetWidget (Variables|Default|GetWidget) _returnvalue)
  (Widget|WidgetHidden true))

(fn SetWidgetWorldRotator
  (Utilities|IsValid (Game|GetPlayerCameraManager 0)
    (:Is%20Valid
      (Transformation|SetWorldRotation (Variables|Default|GetWidget) (Math|Rotator|MakeRotator 0.0 0.0 (.yaw (Math|Rotator|FindLookatRotation (Transformation|GetWorldLocation (Variables|Default|GetWidget)) (Camera|GetCameraLocation (Game|GetPlayerCameraManager 0))))) false false))))

(fn InvertingWidget
  (bind _widget (Variables|Default|GetWidget))
  (bind _widget_2 (Variables|Default|GetWidget))
  (bind _widget_3 (Variables|Default|GetWidget))
  (bind _returnvalue (Transformation|GetWorldLocation _widget_2))
  (bind _bvisible (Variables|/Script/Engine.SceneComponent|GetbVisible _widget))
  (bind _returnvalue_2 (not _bvisible))
  (Rendering|SetVisibility (Variables|Default|GetWidget) _returnvalue_2 false)
  (if _returnvalue_2
    (Collision|SetCollisionEnabled _widget_3 "NoCollision")
    (Rendering|SetVisibility (Variables|Default|GetNiagara) false false)
    (else
      (Collision|SetCollisionEnabled _widget_3 "QueryAndPhysics")
      (Rendering|SetVisibility (Variables|Default|GetNiagara) true false)))
  (Class|NiagaraDataInterfaceArrayFunctionLibrary|SetNiagaraArrayVector (Variables|Default|GetNiagara) "User.PointArray" (Utilities|Array|MakeArray _returnvalue _returnvalue _returnvalue _returnvalue (Transformation|GetWorldLocation (Variables|Default|GetStaticMesh)))))

(fn SetSubItemActorWidget
  (params (Hidden :type Boolean))
  (Widget|WidgetHidden Hidden)
  (bind _subactor (CallFunction|GetThisChildActors))
  (for _array_element _subactor
    (Utilities|IsValid _array_element
      (:Is%20Valid
        (bind _asbp_item_actor (Utilities|Casting|CastToBP_ItemActor _array_element))
        (Widget|SetSubItemActorWidget _asbp_item_actor Hidden)))))

(fn WidgetHidden
  (params (Hidden :type Boolean))
  (bind _returnvalue (not Hidden))
  (bind _widget (Variables|Default|GetWidget))
  (bind _widget_2 (Variables|Default|GetWidget))
  (bind _returnvalue_2 (Transformation|GetWorldLocation _widget))
  (Rendering|SetVisibility (Variables|Default|GetWidget) _returnvalue false)
  (if _returnvalue
    (Collision|SetCollisionEnabled _widget_2 "QueryAndPhysics")
    (Rendering|SetVisibility (Variables|Default|GetNiagara) true false)
    (else
      (Collision|SetCollisionEnabled _widget_2 "NoCollision")
      (Rendering|SetVisibility (Variables|Default|GetNiagara) false false)))
  (Class|NiagaraDataInterfaceArrayFunctionLibrary|SetNiagaraArrayVector (Variables|Default|GetNiagara) "User.PointArray" (Utilities|Array|MakeArray _returnvalue_2 _returnvalue_2 _returnvalue_2 _returnvalue_2 (Transformation|GetWorldLocation (Variables|Default|GetStaticMesh)))))

(fn MeetingParting
  (params (Flip :type Boolean) (Split%20array :type Integer))
  (bind _self self)
  (bind _returnvalue (Actor|GetComponentsByClass _self "/Script/Engine.ChildActorComponent"))
  (bind _returnvalue_2 (Utilities|Array|Length _returnvalue))
  (bind _returnvalue_3 (+ _returnvalue_2 2))
  (bind _returnvalue_4 (/ _returnvalue_3 2))
  (CallFunction|MeetingandParting self (Variables|MeetingandParting|GetDistance) Flip _returnvalue_4 _returnvalue_4 Split%20array))

(fn PlayAnim)

(fn StopAnim)

(fn Reset
  (Reset|ResetSpawnTransform)
  (Anim|StopAnim)
  (Perspective|Perspective false)
  (Widget|SetSubItemActorWidget true)
  (Utilities|FlowControl|Sequence
    (:then_0
      (bind _outactors (Actor|GetAllActorsOfClass "/Game/N_Blueprints/BP_ItemData.BP_ItemData_C"))
      (for _array_element _outactors
        (Utilities|IsValid _array_element
          (:Is%20Valid
            (Actor|DestroyActor _array_element)))))))

(fn ResetSpawnTransform
  (Transformation|SetActorTransform self (Variables|Default|GetThisSpawnTransform))
  (bind _subactor (CallFunction|GetThisChildActors))
  (for _array_element _subactor
    (bind _asbp_item_actor (Utilities|Casting|CastToBP_ItemActor _array_element))
    (Transformation|SetActorTransform _asbp_item_actor (Variables|BP_ItemActor_C|GetThisSpawnTransform _asbp_item_actor))))

(fn AttachtoParentActor
  (Utilities|IsValid (Variables|Default|GetParentActor)
    (:Is%20Valid
      (Transformation|AttachActorToActor self (Variables|Default|GetParentActor) "None" "KeepWorld" "KeepWorld" "KeepWorld" true))))

(event Custom|MeetingAndParting
  (params (Distance :type Float%20%28double-precision%29) (Flip :type Boolean) (Rows :type Integer) (Columns :type Integer) (Split%20array :type Integer))
  (Variables|MeetingAndParting|SetDefaultTransform (Transformation|GetActorTransform))
  (if Flip
    (Development|PrintText "聚合")
    (Collision|SetCollisionEnabled (Variables|Default|GetStaticMesh) "QueryAndPhysics")
    (else
      (Development|PrintText "拆分")
      (Collision|SetCollisionEnabled (Variables|Default|GetStaticMesh) "NoCollision")))
  (bind _subactor (CallFunction|GetThisChildActors))
  (Variables|MeetingAndParting|SetSub%20Actor _subactor)
  (switch int Split%20array
    (:0
      (bind _returnvalue (Class|MyBlueprintFunctionLibrary|ArrangeActorsinHalfCircle3 (Variables|MeetingAndParting|GetSub%20Actor) (Transformation|GetActorLocation) Distance Rows Columns))
      (bind _relativelocations (MeetingAndParting|GetRelativeCoordinates _returnvalue))
      (Variables|MeetingAndParting|SetLoadActorSkewLocation _relativelocations))
    (:1
      (bind _returnvalue_2 (Class|MyBlueprintFunctionLibrary|ArrangeActorsinHalfCircle2 (Variables|MeetingAndParting|GetSub%20Actor) (Transformation|GetActorLocation) Distance Rows Columns))
      (Variables|MeetingAndParting|SetLoadActorSkewLocation _returnvalue_2))
    (:2
      (bind _returnvalue_3 (Class|MyBlueprintFunctionLibrary|ArrangeActorsinHalfCircle1 (Variables|MeetingAndParting|GetSub%20Actor) (Transformation|GetActorLocation) Distance))
      (Variables|MeetingAndParting|SetLoadActorSkewLocation _returnvalue_3)))
  (for (_array_element _array_index) (Variables|MeetingAndParting|GetSub%20Actor)
    (bind _asbp_item_actor (Utilities|Casting|CastToBP_ItemActor _array_element))
    (if (Utilities|Array|IsValidIndex (Variables|MeetingAndParting|GetLoadActorSkewLocation) _array_index)
      (Variables|BP_ItemActor_C|SetSkewTransform _asbp_item_actor (Math|Transform|MakeTransform (Utilities|Array|Get(acopy) (Variables|MeetingAndParting|GetLoadActorSkewLocation) _array_index) (.rotation (Variables|BP_ItemActor_C|GetDefaultTransform _asbp_item_actor)) (.scale (Variables|BP_ItemActor_C|GetDefaultTransform _asbp_item_actor))))
      (CallFunction|SpreadActors _asbp_item_actor Distance Flip Split%20array)))
  (Development|PrintString "聚合拆分计算偏移位置完成" true true "(R=0.000000,G=0.660000,B=1.000000,A=1.000000)" 5.0))

(event Custom|SpreadActors
  (params (Distance :type Float%20%28double-precision%29) (Flip :type Boolean) (Split%20array :type Integer))
  (if Flip
    (bind _alpha (Timeline|excursion Reverse)
      (:Update
        (Transformation|SetActorRelativeTransform self (Math|Transform|Lerp(Transform) (Math|Transform|MakeTransform "0, 0, 0" "0, 0, 0" "1.000000,1.000000,1.000000") (Variables|MeetingAndParting|GetSkewTransform) _alpha) false false)))
    (else
      (Timeline|excursion Play))))
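; BP_ItemData is an actor that shows an item data widget in the world through its widget component.
; On BeginPlay it creates a UMG_ItemData widget, passing its ItemActorID and itself as the owning data actor.
; It assigns that widget to the component and enables query and physics collision on it.
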(event EventBeginPlay
  (|CallParentFunction)
  (bind _returnvalue (UserInterface|CreateWidget "/Game/N_UI/Moudle_1/UMG_ItemData.UMG_ItemData_C" 0 (Variables|Default|GetItemActorID) self))
  (UserInterface|SetWidget (Variables|Default|GetWidget) _returnvalue)
  (Collision|SetCollisionEnabled (Variables|Default|GetWidget) "QueryAndPhysics"))

(event Collision|EventActorBeginOverlap
  (params (OtherActor :type Actor%20Object%20Reference))
  (|CallParentFunction OtherActor) ; This node is disabled and will not be called.\nDrag off pins to build functionality.
)

(event EventTick
  (params (DeltaSeconds :type Float%20%28single-precision%29))
  (|CallParentFunction DeltaSeconds) ; This node is disabled and will not be called.\nDrag off pins to build functionality.
)

(fn ConstructionScript
  (|CallParentFunction))